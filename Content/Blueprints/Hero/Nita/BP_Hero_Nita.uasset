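; Hero Blueprint for Nita that implements her ultimate as a launched projectile skill.
; On UltimateLaunchSkill, the LaunchAimingManager stops the skill montage, sets the release rotation and locks movement orientation, then the ultimate montage plays.
; The montage's notify spawns the ultimate bullet at the RightHand socket, hands it to the aiming manager to launch, unlocks orientation and tells SkillLockComponent the ultimate has finished.
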(event `self.UltimateLaunchSkill`
  (bind (_aimingmanager_flataimingmanager _aimingmanager_launchaimingmanager) (break `AimingManager` (`self.AimingManager`)))
  (bind (_aimingmanager_flataimingmanager_2 _aimingmanager_launchaimingmanager_2) (break `AimingManager` (`self.AimingManager`)))
  (bind (_herotype _normalreleaseoffset _normalmontage _normalmontagesection _normalskillclass _ultimatereleaseoffset _ultimatemontage _ultimatemontagesection) (break `SkillMontage` (`self.HeroSkillMontage`)))
  (`AimingFlat.SkillMontageStop` _aimingmanager_launchaimingmanager_2)
  (`AimingFlat.SetHeroSkillReleaseRotation` _aimingmanager_launchaimingmanager_2 _ultimatereleaseoffset)
  (`AimingFlat.LockMovementOrientRotation` _aimingmanager_launchaimingmanager_2)
  (`|PlayMontage` (`self.Mesh`) _ultimatemontage 1.0 0.0 _ultimatemontagesection
    (:`OnNotifyBegin`
      (bind _returnvalue (`|SpawnActorFromClass` "/Game/Blueprints/Hero/Nita/BP_Bullet_Nita_Ultimate.BP_Bullet_Nita_Ultimate_C" (`KismetMathLibrary.MakeTransform` (`SceneComponent.GetSocketLocation` (`self.Mesh`) "RightHand")) "Undefined" "MultiplyWithRoot" self self))
      (set `self.BulletUltimate` _returnvalue)
      (`AimingLaunch.ReleaseLaunchSkill` _aimingmanager_launchaimingmanager false (`self.BulletUltimate`))
      (`AimingFlat.UnlockMovementOrientRotation` _aimingmanager_launchaimingmanager)
      (`SkillLockComponent.UltimateSkillFinished` (`self.SkillLockComponent`)))))

(fn `UserConstructionScript`
  (`parent.UserConstructionScript`))