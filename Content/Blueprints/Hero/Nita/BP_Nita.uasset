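; Hero Blueprint for Nita that implements the launched ultimate skill.
; UltimateLaunchSkill uses the launch aiming manager to stop the skill montage, set release rotation from the ultimate offset and lock movement-oriented rotation.
; It then plays the ultimate montage, whose notify spawns the ultimate bullet at the right-hand socket, owned by Nita, and stores its reference.
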(event `self.UltimateLaunchSkill`
  (bind (_aimingmanager_flataimingmanager _aimingmanager_launchaimingmanager) (break `AimingManager` (`self.AimingManager`)))
  (bind (_herotype _normalreleaseoffset _normalmontage _normalmontagesection _normalskillclass _ultimatereleaseoffset _ultimatemontage _ultimatemontagesection) (break `SkillMontage` (`self.HeroSkillMontage`)))
  (`AimingFlat.SkillMontageStop` _aimingmanager_launchaimingmanager)
  (`AimingFlat.SetHeroSkillReleaseRotation` _aimingmanager_launchaimingmanager _ultimatereleaseoffset)
  (`AimingFlat.LockMovementOrientRotation` _aimingmanager_launchaimingmanager)
  (`|PlayMontage` (`self.Mesh`) _ultimatemontage 1.0 0.0 _ultimatemontagesection
    (:`OnNotifyBegin`
      (bind _returnvalue (`|SpawnActorFromClass` "/Game/Blueprints/Hero/Nita/BP_Bullet_Nita_Ultimate.BP_Bullet_Nita_Ultimate_C" (`KismetMathLibrary.MakeTransform` (`SceneComponent.GetSocketLocation` (`self.Mesh`) "RightHand")) "Undefined" "MultiplyWithRoot" self null))
      (set `self.BulletUltimate` _returnvalue))))

(fn `UserConstructionScript`
  (`parent.UserConstructionScript`))