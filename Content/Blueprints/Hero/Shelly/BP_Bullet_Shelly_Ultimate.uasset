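; BP_Bullet_Shelly_Ultimate is the bullet Blueprint for Shelly's ultimate, made up of four bullet meshes and four Niagara effects.
; After running the parent construction script, it applies a shared Niagara asset at a fixed enlarged scale and a shared static mesh scaled by BulletWorldScale.
; The event graph holds only disabled placeholder events, so this Blueprint adds construction-time visual setup only.
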(fn `UserConstructionScript`
  (bind _niagara3 (`self.Niagara3`))
  (bind _staticmeshtype (`self.StaticMeshType`))
  (`parent.UserConstructionScript`)
  (`NiagaraComponent.SetAsset` _niagara3 (`self.NiagaraType`) true)
  (`NiagaraComponent.SetAsset` (`self.Niagara1`) (`self.NiagaraType`) true)
  (`NiagaraComponent.SetAsset` (`self.Niagara2`) (`self.NiagaraType`) true)
  (`NiagaraComponent.SetAsset` (`self.Niagara`) (`self.NiagaraType`) true)
  (`SceneComponent.SetWorldScale3D` _niagara3 (5.0 5.0 5.0))
  (`SceneComponent.SetWorldScale3D` (`self.Niagara2`) (5.0 5.0 5.0))
  (`SceneComponent.SetWorldScale3D` (`self.Niagara1`) (5.0 5.0 5.0))
  (`SceneComponent.SetWorldScale3D` (`self.Niagara`) (5.0 5.0 5.0))
  (`|ExecutionSequence`
    (:`then_0`
      (`StaticMeshComponent.SetStaticMesh` (`self.Bullet`) _staticmeshtype)
      (`SceneComponent.SetWorldScale3D` (`self.Bullet`) (`self.BulletWorldScale`))
      (`SceneComponent.SetWorldScale3D` (`self.Bullet1`) (`self.BulletWorldScale`))
      (`SceneComponent.SetWorldScale3D` (`self.Bullet2`) (`self.BulletWorldScale`))
      (`SceneComponent.SetWorldScale3D` (`self.Bullet3`) (`self.BulletWorldScale`)))
    (:`then_1`
      (`StaticMeshComponent.SetStaticMesh` (`self.Bullet1`) _staticmeshtype))
    (:`then_2`
      (`StaticMeshComponent.SetStaticMesh` (`self.Bullet2`) _staticmeshtype))
    (:`then_3`
      (`StaticMeshComponent.SetStaticMesh` (`self.Bullet3`) _staticmeshtype))))