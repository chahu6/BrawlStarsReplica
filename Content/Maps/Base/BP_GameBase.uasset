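; BP_GameBase is a controller Blueprint that spawns and possesses the player's chosen hero when play begins on the local player controller.
; It reads HeroType from BP_GameInstance, falling back to BP_Hero_Colt if none is valid.
; The hero spawns at the location of the first BP_PlayerStart found, as the loop breaks after one spawn.
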(event `self.ReceiveBeginPlay`
  (if (`self.IsLocalPlayerController`)
    (`self.GetHeroTypeAndSpawn`)))

(event `GetHeroTypeAndSpawn`
  (bind _asbp_game_instance (cast `/Game/Blueprints/BP_GameInstance` (`GameplayStatics.GetGameInstance`)))
  (bind _herotype (`/Game/Blueprints/BP_GameInstance.HeroType` _asbp_game_instance)
    (:`then`
      (set `self.HeroType` _herotype))
    (:`else`
      (set `self.HeroType` "/Game/Blueprints/Hero/Colt/BP_Hero_Colt.BP_Hero_Colt_C")))
  (`self.SpawnHero`))

(event `SpawnHero`
  (bind _outactors (`GameplayStatics.GetAllActorsOfClass` "/Game/Maps/Base/BP_PlayerStart.BP_PlayerStart_C"))
  (for _array_element _outactors
    (`|ExecutionSequence`
      (:`then_0`
        (bind _returnvalue (`|SpawnActorFromClass` (`self.HeroType`) (`KismetMathLibrary.MakeTransform` (`self.K2_GetActorLocation` _array_element)) "Undefined" "MultiplyWithRoot" self null))
        (`self.Possess` _returnvalue))
      (:`then_1`
        (break)))))

(fn `UserConstructionScript`)