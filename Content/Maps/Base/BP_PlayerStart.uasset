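; BP_PlayerStart is a map spawn point marker that tracks whether a hero is occupying it.
; The construction script sets up a small, collision-free marker mesh with an "available" material and flags the point as available.
; Sphere overlaps with HeroBase actors toggle IsAvailable and swap the material to match, without counting overlaps, so any hero leaving marks it available.
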(event `self.Sphere.OnComponentBeginOverlap`
  (params (OverlappedComponent :type "PrimitiveComponent Object Reference") (OtherActor :type "Actor Object Reference") (OtherComp :type "PrimitiveComponent Object Reference") (OtherBodyIndex :type Integer) (bFromSweep :type Boolean) (SweepResult :type "HitResult Structure (by ref)"))
  (cast `HeroBase` OtherActor)
  (set `self.bIsAvailable` false)
  (`PrimitiveComponent.SetMaterial` (`self.StaticMesh`) 0 "/Game/Assets/Map/Base/Asset/MI_Map_PlayerStartPoint_NotAvaliable.MI_Map_PlayerStartPoint_NotAvaliable"))

(event `self.Sphere.OnComponentEndOverlap`
  (params (OverlappedComponent :type "PrimitiveComponent Object Reference") (OtherActor :type "Actor Object Reference") (OtherComp :type "PrimitiveComponent Object Reference") (OtherBodyIndex :type Integer))
  (cast `HeroBase` OtherActor)
  (set `self.bIsAvailable` true)
  (`PrimitiveComponent.SetMaterial` (`self.StaticMesh`) 0 "/Game/Assets/Map/Base/Asset/MI_Map_PlayerStartPoint_Avaliable.MI_Map_PlayerStartPoint_Avaliable"))

(fn `UserConstructionScript`
  (bind _staticmesh (`self.StaticMesh`))
  (`StaticMeshComponent.SetStaticMesh` _staticmesh "/Game/Assets/Map/Base/Asset/SM_Map_PlayerStartPoint.SM_Map_PlayerStartPoint")
  (`PrimitiveComponent.SetMaterial` _staticmesh 0 "/Game/Assets/Map/Base/Asset/MI_Map_PlayerStartPoint_Avaliable.MI_Map_PlayerStartPoint_Avaliable")
  (`PrimitiveComponent.SetCollisionEnabled` _staticmesh "NoCollision")
  (`SceneComponent.SetWorldScale3D` _staticmesh (0.5 0.5 0.5))
  (set `self.bIsAvailable` true))