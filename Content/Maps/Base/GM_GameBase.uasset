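; Base game mode that starts the match once the expected player count from BP_GameInstance has joined.
; The last player's pawn possession triggers a warmup delay, then start sounds, AI spawning, input enabling and background music.
; SpawnAI places six random DT_Hero heroes at available BP_PlayerStarts, copying each start's team to pawn and PlayerState.
; Music is picked randomly from the current level's DT_GameMusic list.
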(event `self.K2_PostLogin`
  (params (NewPlayer :type "PlayerController Object Reference"))
  ;[1 1 1] Game Manager
  (bind _aspc_game_base (cast `/Game/Maps/Base/PC_GameBase` NewPlayer))
  (`/Game/Maps/Base/PC_GameBase.GameIntroduction` _aspc_game_base)
  (`/Engine/EditorBlueprintResources/StandardMacros.IncrementInt` (`self.PlayerNumber`)
    (:`  `
      (if (`self.CheckPlayerNumber`)
        (add `Controller.OnPossessedPawnChanged` NewPlayer (delegate `OnPossessedPawnChanged_Event`))))))

(event `OnPossessedPawnChanged_Event`
  (params (OldPawn :type "Pawn Object Reference") (NewPawn :type "Pawn Object Reference"))
  ;[1 1 1] Game Manager
  (`self.GameBeginPlay`)
  (remove `Controller.OnPossessedPawnChanged` (stale `self.K2_PostLogin` NewPlayer) (delegate `OnPossessedPawnChanged_Event`)))

(event `PlayBackgroundMusic`
  ;[1 1 1] Game Music Manager
  (bind _music (`self.GetGameBackGroundMusic`))
  (bind _returnvalue (`GameplayStatics.CreateSound2D` _music 1.0 1.0 0.0 null))
  (bind _output_get (set `self.BackgroundMusic` _returnvalue))
  (`AudioComponent.Play` _output_get 0.0))

(event `GameBeginPlay`
  ;[1 1 1] Game Manager
  (`KismetSystemLibrary.Delay` (`self.WarmupTime`))
  (bind _returnvalue (`self.GetNumPlayers`))
  (for _index (range _returnvalue)
    (bind _aspc_game_base (cast `/Game/Maps/Base/PC_GameBase` (`GameplayStatics.GetPlayerController` _index)))
    (`/Game/Maps/Base/PC_GameBase.PlayGameBeginSound` _aspc_game_base))
  (`self.SpawnAI` 6)
  (`self.PlayerInputEnable`)
  (`KismetSystemLibrary.Delay` 1.0)
  (`self.PlayBackGroundMusic`))

(event `PlayerInputDisable`
  ;[1 1 1] Player Input Manager
  (bind _returnvalue (`self.GetNumPlayers`))
  (for _index (range _returnvalue)
    (bind _aspc_game_base (cast `/Game/Maps/Base/PC_GameBase` (`GameplayStatics.GetPlayerController` _index)))
    (`/Game/Maps/Base/PC_GameBase.PlayerControllerInputDisable` _aspc_game_base)))

(event `PlayerInputEnable`
  ;[1 1 1] Player Input Manager
  (bind _returnvalue (`self.GetNumPlayers`))
  (for _index (range _returnvalue)
    (bind _aspc_game_base (cast `/Game/Maps/Base/PC_GameBase` (`GameplayStatics.GetPlayerController` _index)))
    (`/Game/Maps/Base/PC_GameBase.PlayerControllerInputEnable` _aspc_game_base)))

(fn `CheckPlayerNumber`
  (returns (ReturnValue :type Boolean))
  (bind _asbp_game_instance (cast `/Game/Blueprints/BP_GameInstance` (`GameplayStatics.GetGameInstance`)))
  (return (>= (`self.PlayerNumber`) (`/Game/Blueprints/BP_GameInstance.PlayerNumber` _asbp_game_instance))))

(fn `GetGameBackGroundMusic`
  (returns (Music :type "SoundBase Object Reference"))
  (locals (L_CurrentLevelName :type String) (L_MusicList :type "Array of SoundBase Object Reference"))
  (bind _returnvalue (`GameplayStatics.GetCurrentLevelName` true))
  (set `local.L_CurrentLevelName` _returnvalue)
  (bind _outrownames (`DataTableFunctionLibrary.GetDataTableRowNames` "/Game/Maps/Base/Data/DT_GameMusic.DT_GameMusic"))
  (for _array_element _outrownames
    (bind _returnvalue_2 (`|GetDataTableRow` "/Game/Maps/Base/Data/DT_GameMusic.DT_GameMusic" _array_element)
      (:`then`
        (bind (_levelname _music) (break `/Game/Maps/Base/Data/FGameMusic` _returnvalue_2))
        (if (`KismetStringLibrary.EqualEqual_StrStr` (`|GetEnumeratorNameAsString` _levelname) (`local.L_CurrentLevelName`))
          (set `local.L_MusicList` _music)))))
  (return (`/Game/Blueprints/BP_BrawlStarsFunctionLibrary.FL_GetRandomSound` (`local.L_MusicList`))))

(fn `SpawnAI`
  (params (Amount :type Integer))
  (locals (L_PlayerStartPoint :type "/Game/Maps/Base/BP_PlayerStart Object Reference") (L_SpawnedHeroClass :type "HeroBase Class Reference") (L_SpawnedHero :type "HeroBase Object Reference") (L_AIAmountRemain :type Integer))
  (bind _l_playerstartpoint (`local.L_PlayerStartPoint`))
  (bind _l_spawnedhero (`local.L_SpawnedHero`))
  (set `local.L_AIAmountRemain` Amount)
  (bind _outactors (`GameplayStatics.GetAllActorsOfClass` "/Game/Maps/Base/BP_PlayerStart.BP_PlayerStart_C"))
  (for _array_element _outactors
    (if (> (`local.L_AIAmountRemain`) 0)
      (set `local.L_PlayerStartPoint` _array_element)
      (if (`/Game/Maps/Base/BP_PlayerStart.bIsAvailable` _l_playerstartpoint)
        (set `/Game/Maps/Base/BP_PlayerStart.bIsAvailable` false _l_playerstartpoint)
        (bind _outrownames (`DataTableFunctionLibrary.GetDataTableRowNames` "/Game/Blueprints/Hero/Data/DT_Hero.DT_Hero"))
        (bind _returnvalue (`|GetDataTableRow` "/Game/Blueprints/Hero/Data/DT_Hero.DT_Hero" (`|GetArrayItem` _outrownames (`KismetMathLibrary.RandomInteger` (`KismetArrayLibrary.Array_Length` _outrownames))))
          (:`then`
            (set `local.L_SpawnedHeroClass` (`.HeroType` (break `HeroAttribute` _returnvalue)))
            (bind _returnvalue_2 (`|SpawnActorFromClass` (`local.L_SpawnedHeroClass`) (`KismetMathLibrary.MakeTransform` (`self.K2_GetActorLocation` (`local.L_PlayerStartPoint`))) "Undefined" "MultiplyWithRoot" null null))
            (set `local.L_SpawnedHero` _returnvalue_2)
            (set `HeroBase.TeamType` (`/Game/Maps/Base/BP_PlayerStart.TeamType` (`local.L_PlayerStartPoint`)) (`local.L_SpawnedHero`))
            (bind _asaic_game_base (cast `/Game/Blueprints/AI/AIC_GameBase` (`Pawn.GetController` _l_spawnedhero)))
            (bind _asps_game_base (cast `/Game/Maps/Base/PS_GameBase` (`Controller.PlayerState` _asaic_game_base))
              (:`then`
                (set `/Game/Maps/Base/PS_GameBase.TeamType` (`HeroBase.TeamType` _l_spawnedhero) _asps_game_base)
                (`/Engine/EditorBlueprintResources/StandardMacros.DecrementInt` (`local.L_AIAmountRemain`)))
              (:`CastFailed`
                (`KismetSystemLibrary.PrintString` "AI控制器没有勾选bWantsPlayerState！"))))))
      (else
        (break)))))

(fn `UserConstructionScript`)