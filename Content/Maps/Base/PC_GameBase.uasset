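; Base player controller that spawns and possesses the player's hero at a team start point.
; On BeginPlay the local controller reads hero and team from the game instance, falling back to Colt, and writes the team to the player state.
; It claims the first available matching BP_PlayerStart, spawns the hero there and possesses it.
; On local possession, Team B pawns and controller are yawed 180 degrees; GameIntroduction is an empty stub.
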(event `self.ReceiveBeginPlay`
  (if (`self.IsLocalPlayerController`)
    (`self.GetHeroTypeAndSpawn`)))

(event `GetHeroTypeAndSpawn`
  (bind _asbp_game_instance (cast `/Game/Blueprints/BP_GameInstance` (`GameplayStatics.GetGameInstance`)))
  (bind _herotype (`/Game/Blueprints/BP_GameInstance.HeroType` _asbp_game_instance)
    (:`then`
      (set `self.HeroType` _herotype))
    (:`else`
      (set `self.HeroType` "/Game/Blueprints/Hero/Colt/BP_Hero_Colt.BP_Hero_Colt_C")))
  (set `self.TeamType` (`/Game/Blueprints/BP_GameInstance.TeamType` _asbp_game_instance))
  (`self.SetHeroTypeAndTeamType`))

(event `SetHeroTypeAndTeamType`
  (bind _asps_game_base (cast `/Game/Maps/Base/PS_GameBase` (`self.PlayerState`)))
  (set `/Game/Maps/Base/PS_GameBase.TeamType` (`self.TeamType`) _asps_game_base)
  (`self.SpawnHero`))

(event `SpawnHero`
  ;[1 1 1] Spawn Hero
  (bind _outactors (`GameplayStatics.GetAllActorsOfClass` "/Game/Maps/Base/BP_PlayerStart.BP_PlayerStart_C"))
  (for _array_element _outactors
    (if (and (`/Game/Maps/Base/BP_PlayerStart.bIsAvailable` _array_element) (`|EnumEquality` (`self.TeamType`) (`/Game/Maps/Base/BP_PlayerStart.TeamType` _array_element)))
      (set `/Game/Maps/Base/BP_PlayerStart.bIsAvailable` false _array_element)
      (`|ExecutionSequence`
        (:`then_0`
          (bind _returnvalue (`|SpawnActorFromClass` (`self.HeroType`) (`KismetMathLibrary.MakeTransform` (`self.K2_GetActorLocation` _array_element)) "Undefined" "MultiplyWithRoot" self null))
          (`self.Possess` _returnvalue))
        (:`then_1`
          (break))))))

(event `self.ReceivePossess`
  (params (PossessedPawn :type "Pawn Object Reference"))
  (if (`self.IsLocalPlayerController`)
    (`self.SetPlayerControllerRotationByTeamType`)))

(event `SetPlayerControllerRotationByTeamType`
  (bind _returnvalue (`self.K2_GetPawn`))
  (if (`|EnumEquality` (`self.TeamType`) "ET_TeamB")
    (`/Engine/EditorBlueprintResources/StandardMacros.IsValid` _returnvalue
      (:`Is Valid`
        (`self.K2_SetActorRotation` _returnvalue (struct :`Yaw` 180.0) false)
        (`self.SetInitialLocationAndRotation` (`self.K2_GetActorLocation` _returnvalue) (`KismetMathLibrary.MakeRotator` 0.0 0.0 180.0))))))

(event `GameIntroduction`)

(fn `UserConstructionScript`)