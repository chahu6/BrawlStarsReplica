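; Player controller for the login/lobby map, handling menu music, the exhibition camera view and hero selection.
; Next/Last events cycle a wrapping index that excludes the final array entry; SwitchHero shows only that hero with its attachments and saves its class to BP_GameInstance.
; A helper gathers display transforms from BP_ExhibitionPoint actors with a fixed rotation.
; Starting matchmaking replaces the current widget with the match widget.
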(event `self.ReceiveBeginPlay`
  (if (`self.IsLocalController`)
    (`GameplayStatics.PlaySound2D` "/Game/Assets/Sound/Login/brawl_stars_menu_01.brawl_stars_menu_01" 0.4 1.0 0.0 null null)))

(event `UseExhibitinoCamera`
  (bind _exhibitioncamera (`self.ExhibitionCamera`)
    (:`then`
      (`self.SetViewTargetWithBlend` self _exhibitioncamera 0.0 "VTBlend_Linear" 0.0 false))
    (:`else`)))

(event `NextHero`
  ;[1 1 1] Switch Hero
  (set `self.CurrentHeroIndex` (mod (+ (`self.CurrentHeroIndex`) 1) (- (`KismetArrayLibrary.Array_Length` (`self.ExhibitionHero`)) 1)))
  (`self.SwitchHero`))

(event `LastHero`
  (bind _returnvalue (- (`KismetArrayLibrary.Array_Length` (`self.ExhibitionHero`)) 1))
  ;[1 1 1] Switch Hero
  (set `self.CurrentHeroIndex` (mod (+ (- (`self.CurrentHeroIndex`) 1) _returnvalue) _returnvalue))
  (`self.SwitchHero`))

(event `StartGameMatching`
  (`self.ShowMatchingWidget`))

(event `ShowMatchingWidget`
  (bind _wbp_login (`self.WBP_Login`)
    (:`then`
      (`Widget.RemoveFromParent` _wbp_login))
    (:`else`
      _))
  (bind _returnvalue (`|CreateWidget` "/Game/Blueprints/UI/Base/WBP_GameBase_Match.WBP_GameBase_Match_C" self))
  (bind _output_get (set `self.WBP_Login` _returnvalue))
  (`UserWidget.AddToViewport` _output_get 0))

(fn `GetHeroExhibitionPointTransfrom`
  (`KismetArrayLibrary.Array_Clear` (`self.ExhibitionPointTransfrom`))
  (bind _outactors (`GameplayStatics.GetAllActorsOfClass` "/Game/Maps/Base/BP_ExhibitionPoint.BP_ExhibitionPoint_C"))
  (for _array_element _outactors
    (bind (_returnvalue_location _returnvalue_rotation _returnvalue_scale) (`KismetMathLibrary.BreakTransform` (`self.GetTransform` _array_element)))
    (`KismetArrayLibrary.Array_Add` (`self.ExhibitionPointTransfrom`) (`KismetMathLibrary.MakeTransform` _returnvalue_location (struct :`Yaw` 180.0) _returnvalue_scale)))
  (if (== (`KismetArrayLibrary.Array_Length` (`self.ExhibitionPointTransfrom`)) 0)
    (`KismetSystemLibrary.PrintString` "未找到！！！")))

(fn `SwitchHero`
  (bind _output (`|GetArrayItem` (`self.ExhibitionHero`) (`self.CurrentHeroIndex`)))
  (for _array_element (`self.ExhibitionHero`)
    (bind _outactors (`self.GetAttachedActors` _array_element true false))
    (`self.SetActorHiddenInGame` _outactors true)
    (`self.SetActorEnableCollision` _outactors false)
    (`self.SetActorHiddenInGame` _array_element true)
    (`self.SetActorEnableCollision` _array_element false))
  (`self.SetActorHiddenInGame` _output false)
  (`self.SetActorHiddenInGame` (`self.GetAttachedActors` _output true false) false)
  (set `self.CurrentHeroType` (`GameplayStatics.GetObjectClass` _output))
  (bind _asbp_game_instance (cast `/Game/Blueprints/BP_GameInstance` (`GameplayStatics.GetGameInstance`)))
  (set `/Game/Blueprints/BP_GameInstance.HeroType` (`self.CurrentHeroType`) _asbp_game_instance))

(fn `UserConstructionScript`
  (set `self.DefaultHeroType` "/Game/Blueprints/Hero/Shelly/BP_Hero_Shelly.BP_Hero_Shelly_C"))