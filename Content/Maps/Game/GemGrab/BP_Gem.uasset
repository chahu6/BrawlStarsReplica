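; BP_Gem is a collectible gem actor in the GemGrab map folder, launched with projectile movement and picked up by heroes.
; It plays a spawn sound on BeginPlay, and a SetVelocity event sets the projectile's velocity in local space.
; When a HeroBase overlaps PickupDetect, it plays a 2D pickup sound and destroys itself, with no scoring here.
; The construction script scales the sphere and a larger pickup detector.
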(event `self.ReceiveBeginPlay`
  (`GameplayStatics.PlaySoundAtLocation` "/Game/Assets/Sound/Game/GemGrab/pickup_spawn_03.pickup_spawn_03" (`self.K2_GetActorLocation`) (struct) 1.0 1.0 0.0 null null null null))

(event `SetVelocity`
  (params (InVelocity :type "Vector Structure"))
  (`ProjectileMovementComponent.SetVelocityInLocalSpace` (`self.ProjectileMovement`) InVelocity))

(event `self.PickupDetect.OnComponentBeginOverlap`
  (params (OverlappedComponent :type "PrimitiveComponent Object Reference") (OtherActor :type "Actor Object Reference") (OtherComp :type "PrimitiveComponent Object Reference") (OtherBodyIndex :type Integer) (bFromSweep :type Boolean) (SweepResult :type "HitResult Structure (by ref)"))
  (cast `HeroBase` OtherActor)
  (`GameplayStatics.PlaySound2D` "/Game/Assets/Sound/Game/GemGrab/get_pickup_06.get_pickup_06" 1.0 1.0 0.0 null null)
  (`self.K2_DestroyActor`))

(fn `UserConstructionScript`
  (`SceneComponent.SetWorldScale3D` (`self.Sphere`) (2.0 2.0 2.0))
  (`SceneComponent.SetWorldScale3D` (`self.PickupDetect`) (3.0 3.0 3.0)))