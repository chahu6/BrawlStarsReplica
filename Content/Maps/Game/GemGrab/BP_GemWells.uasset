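; BP_GemWells is a gem spawner actor for the GemGrab map that periodically produces BP_Gem actors.
; A looping timer started on BeginPlay uses SpawnedSpeed as its interval and spawns each gem just above the well, adjusting for collisions.
; Each valid gem is launched upward with a random horizontal spread, and the Niagara effect is restarted with each launch.
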(event `self.ReceiveBeginPlay`
  (`KismetSystemLibrary.K2_SetTimerDelegate` (delegate `SpawnGem`) (`self.SpawnedSpeed`) true))

(event `SpawnGem`
  (bind (_returnvalue_x _returnvalue_y _returnvalue_z) (`KismetMathLibrary.BreakVector` (`self.K2_GetActorLocation`)))
  (bind _returnvalue (`|SpawnActorFromClass` "/Game/Maps/Game/GemGrab/BP_Gem.BP_Gem_C" (`KismetMathLibrary.MakeTransform` (`KismetMathLibrary.MakeVector` _returnvalue_x _returnvalue_y (+ _returnvalue_z 100.0))) "AdjustIfPossibleButAlwaysSpawn" "MultiplyWithRoot" null null))
  (`/Engine/EditorBlueprintResources/StandardMacros.IsValid` _returnvalue
    (:`Is Valid`
      (`/Game/Maps/Game/GemGrab/BP_Gem.SetVelocity` _returnvalue (* (+ (`KismetMathLibrary.GetUpVector` (struct)) (`KismetMathLibrary.MakeVector` (`KismetMathLibrary.RandomFloatInRange` -1.0 1.0) (`KismetMathLibrary.RandomFloatInRange` -1.0 1.0))) 300.0))
      (`ActorComponent.Activate` (`self.Niagara`) true))))

(fn `UserConstructionScript`)