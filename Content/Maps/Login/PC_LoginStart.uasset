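; Player controller for the login map that sets up a hero showcase and the login UI on BeginPlay.
; It spawns every DT_Hero entry at the first exhibition point, hidden and without collision along with attached actors, then calls SwitchHero.
; It then finds the BP_ExhibitionCamera, switches to it, and, for the local controller only, adds WBP_LoginBase with a visible cursor.
; The UI-only input mode node is left unconnected.
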(event `self.ReceiveBeginPlay`
  (`parent.ReceiveBeginPlay`)
  (`self.SpawnHeroForExhibition`)
  (bind _outactors (`GameplayStatics.GetAllActorsOfClass` "/Game/Maps/Base/BP_ExhibitionCamera.BP_ExhibitionCamera_C"))
  (set `self.ExhibitionCamera` (`|GetArrayItem` _outactors))
  (`self.UseExhibitinoCamera`)
  (`self.InitLoginUMG`))

(event `SpawnHeroForExhibition`
  ;[1 1 1] 生成Hero并Show
  (set `self.CurrentHeroType` (`self.DefaultHeroType`))
  (`self.GetHeroExhibitionPointTransfrom`)
  (bind _outrownames (`DataTableFunctionLibrary.GetDataTableRowNames` "/Game/Blueprints/Hero/Data/DT_Hero.DT_Hero"))
  (for _array_element _outrownames
    (bind _returnvalue (`|GetDataTableRow` "/Game/Blueprints/Hero/Data/DT_Hero.DT_Hero" _array_element)
      (:`then`
        (bind _returnvalue_2 (`|SpawnActorFromClass` (break `HeroAttribute` _returnvalue) (`|GetArrayItem` (`self.ExhibitionPointTransfrom`)) "Undefined" "MultiplyWithRoot" null null))
        (bind _outactors (`self.GetAttachedActors` _returnvalue_2 true false))
        (`self.SetActorHiddenInGame` _outactors true)
        (`self.SetActorEnableCollision` _outactors false)
        (`self.SetActorHiddenInGame` _returnvalue_2 true)
        (`self.SetActorEnableCollision` _returnvalue_2 false)
        (`KismetArrayLibrary.Array_AddUnique` (`self.ExhibitionHero`) _returnvalue_2))))
  (`self.SwitchHero`))

(event `InitLoginUMG`
  ;[1 1 1] UI Manager
  (if (`self.IsLocalController`)
    (bind _returnvalue (`|CreateWidget` "/Game/Blueprints/UI/Login/WBP_LoginBase.WBP_LoginBase_C" self))
    (set `self.WBP_Login` _returnvalue)
    (`UserWidget.AddToViewport` _returnvalue 0)
    (set `self.bShowMouseCursor` true)))

(fn `UserConstructionScript`
  (`parent.UserConstructionScript`))